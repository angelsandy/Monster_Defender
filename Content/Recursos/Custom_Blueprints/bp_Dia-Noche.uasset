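; Day-night cycle actor that rotates a directional light to move the sun across the sky.
; Tick plays a timeline whose rotation curve, scaled by a speed variable and offset by an initial position, sets the light source's pitch.
; Each timeline update also refreshes the sky sphere's sun direction to match the light.
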(event EventBeginPlay)

(event Collision|EventActorBeginOverlap
  (params (OtherActor :type Actor%20Object%20Reference)))

(event EventTick
  (params (DeltaSeconds :type Float%20%28single-precision%29))
  ;[1 1 1] Ciclo De Dia y Noche
  (bind _rotacion_24min_360 (Timeline|tlRotacion Play)
    (:Update
      (Transformation|SetActorRotation (Variables|Default|GetLightSource) (Math|Rotator|MakeRotator 0.0 (+ (Variables|Default|GetPosicionInicial) (* _rotacion_24min_360 (Math|Conversions|ToFloat(Integer) (Variables|Default|GetVelocidad)))) 0.0))
      (Default|UpdateSunDirection (Variables|Default|GetSkySphere)))))

(fn ConstructionScript)